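; BP_Sujet1 is an integration exercise actor that lays out one named spot and one spawned character per student.
; The construction script adds centered text labels with each student's enum name in a centered row along Y, alternating in height.
; On BeginPlay, it asks each student's exercise subsystem, via IntegrationSubsystem, to spawn that student's character at the matching world-axis offset, shifted along X.
; An unconnected square-grid label layout remains in the construction script.
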(event EventBeginPlay
  (bind _returnvalue (Class|CommonFunctionLibrary|GetAllStudents))
  (for (_array_element _array_index) _returnvalue
    (bind _returnvalue_2 (Class|IntegrationSubsystem|GetExerciceSubSystembyStudent (Subsystems|GetIntegrationSubsystem) _array_element))
    (Class|ExerciceSubsystemInterface|SpawnStudentCharacter _returnvalue_2 (Math|Transform|MakeTransform (+ (Transformation|GetActorLocation) (Math|Vector|MakeVector 1e+02 (- (* _array_index 2e+02) (* (/ (Utilities|Array|Length _returnvalue) 2) 2e+02)) (* (Math|Integer|%(Integer) _array_index 2) 25.0))) "0, 0, 0" "1,1,1"))))

(fn ConstructionScript
  (bind _returnvalue (Class|CommonFunctionLibrary|GetAllStudents))
  (for (_array_element _array_index) _returnvalue
    (bind _returnvalue_2 (AddComponent|AddTextRenderComponent false (Math|Transform|MakeTransform (Math|Vector|MakeVector 0.0 (- (* _array_index 2e+02) (* (/ (Utilities|Array|Length _returnvalue) 2) 2e+02)) (* (Math|Integer|%(Integer) _array_index 2) 25.0)) "0,180.000000, 0" "1,1,1")))
    (Rendering|Components|TextRender|SetText _returnvalue_2 (Utilities|Text|ToText(String) (Utilities|String|EnumtoString _array_element)))
    (Rendering|Components|TextRender|SetHorizontalAlignment _returnvalue_2 "EHTA_Center")))